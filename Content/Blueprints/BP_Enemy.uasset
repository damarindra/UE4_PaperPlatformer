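; BP_Enemy is an AI-controlled enemy character that walks to a random point in the level when play begins.
; On BeginPlay it gathers every TargetPoint actor into a Waypoints array, picks one at random and uses SimpleMoveToLocation through its AI controller.
; The move is issued only once, with no repeat patrol, and the Tick, overlap and construction logic are empty.
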(event `self.ReceiveBeginPlay`
  (bind _waypoints (`self.Waypoints`))
  (bind _outactors (`GameplayStatics.GetAllActorsOfClass` "/Script/Engine.TargetPoint"))
  (set `self.Waypoints` _outactors)
  (`AIBlueprintHelperLibrary.SimpleMoveToLocation` (`AIBlueprintHelperLibrary.GetAIController` self) (`self.K2_GetActorLocation` (`|GetArrayItem` _waypoints (`KismetMathLibrary.RandomInteger` (`KismetArrayLibrary.Array_Length` _waypoints))))))

(event `self.ReceiveTick`
  (params (DeltaSeconds :type "Float (single-precision)")))

(fn `UserConstructionScript`)